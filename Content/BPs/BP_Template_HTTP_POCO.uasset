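; Template actor that runs a POCO-based HTTP server and answers incoming API requests.
; BeginPlay spawns an HTTP_Server_POCO on a fixed API URI and binds its request delegate to a parse function.
; That function prints the client address and replies with a placeholder string and custom header.
; A disconnected branch holds unused debug printing of host, headers, URI, body and query.
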(event Custom|DelegateHttpRequest_Event
  (params (Request :type Http%20Request%20Poco%20Object%20Reference))
  (CallFunction|FParseRequest Request))

(event EventBeginPlay
  (bind _returnvalue (Game|SpawnActorfromClass "/Script/FF_HTTP_POCO.HTTP_Server_POCO" (Math|Transform|MakeTransform "0, 0, 0" "0, 0, 0" "1.000000,1.000000,1.000000") "Undefined" "MultiplyWithRoot" 0 "/api/poco/v1/" "SRV_POCO_" 8081 8453 1 0))
  (bind _output_get (Variables|Default|SetServer_POCO _returnvalue))
  (EventDispatchers|AssignDelegateHttpRequest _output_get (delegate Custom|DelegateHttpRequest_Event)))

(fn ConstructionScript)

(fn FParseRequest
  (params (In_Request :type Http%20Request%20Poco%20Object%20Reference))
  (Utilities|IsValid In_Request
    (:Is%20Valid
      (LocalVariables|SetLOC_Request In_Request)
      (bind _out_address (Class|HttpRequestPoco|GetClientAddress (LocalVariables|GetLOC_Request)))
      (Development|PrintString (Utilities|String|Append "Client Address = " _out_address) true true "(R=0.000000,G=0.660000,B=1.000000,A=1.000000)" 3e+01)
      (Class|HttpRequestPoco|SendResponseString (LocalVariables|GetLOC_Request) (Utilities|Map|MakeMap "eray" "ezgi") "anan" "OK_200" "Text_Plain" true)
      (return))
    (:Is%20Not%20Valid
      (return))))