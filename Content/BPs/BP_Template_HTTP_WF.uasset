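; Template actor that runs an HTTP server through the FF_HTTP_WF plugin.
; On BeginPlay it resolves the web root and 404 page from the plugin's resources folder, then spawns an HTTP_Server_WF with those paths and a dynamic API URI.
; It binds the server's request delegate, which prints each request URI on screen and replies with a Hello World HTML page.
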(event Custom|DelegateHttpRequest_Event
  (params (Request :type Http%20Request%20Wf%20Object%20Reference))
  (bind _out_uri (Class|HttpRequestWf|GetRequestUri Request))
  (Development|PrintString _out_uri true true "(R=0.000000,G=0.660000,B=1.000000,A=1.000000)" 3e+01)
  (Class|HttpRequestWf|SendResponse Request "<html>Hello World!</html>"))

(event EventBeginPlay
  (bind (_outbasedir _returnvalue) (Class|PluginBlueprintLibrary|GetPluginBaseDir "FF_HTTP_WF"))
  (if _returnvalue
    (Variables|General|SetPath_Root (Class|BlueprintPathsLibrary|MakePlatformFilename (Class|KismetSystemLibrary|ConverttoAbsolutePath (Utilities|String|Append _outbasedir "/Resources/wwwroot/root/"))))
    (Variables|General|SetPath_404 (Class|KismetSystemLibrary|ConverttoAbsolutePath (Utilities|String|Append _outbasedir "/Resources/wwwroot/404.html"))))
  (bind _returnvalue_2 (Game|SpawnActorfromClass "/Script/FF_HTTP_WF.HTTP_Server_WF" (Math|Transform|MakeTransform "0, 0, 0" "0, 0, 0" "1.000000,1.000000,1.000000") "Undefined" "MultiplyWithRoot" 0 (Variables|General|GetPath_Root) (Variables|General|GetPath_404) 8081 8453 "/dyn" "LibWebSocket" 0))
  (bind _output_get (Variables|Default|SetServer_NGH _returnvalue_2))
  (EventDispatchers|AssignDelegateHttpRequest _output_get (delegate Custom|DelegateHttpRequest_Event)))

(fn ConstructionScript)